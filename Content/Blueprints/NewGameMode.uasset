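; Game mode for a click-the-sphere shooting game that moves from ShootingSceneBlue to ShootingSceneRed at ten points.
; BeginPlay shows the cursor, blocks look and move input, builds the score widget and loads or creates the HighScore save.
; Tick hit-tests the mouse against the sphere's projected screen position, then scores and respawns it at a cycling Y position.
; EndPlay passes the score to the save object and writes it.
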(event EventBeginPlay
  (bind _returnvalue (Game|GetPlayerController 0))
  ;[1 1 1] Enable cursor/disable input
  (Variables|/Script/Engine.PlayerController|SetbShowMouseCursor _returnvalue true)
  (Input|SetIgnoreLookInput _returnvalue true)
  (Input|SetIgnoreMoveInput _returnvalue true)
  ;[1 1 1] Create score widget
  (bind _returnvalue_2 (UserInterface|CreateWidget "/Game/BaseWorld/Score.Score_C"))
  (bind _output_get (Variables|Default|SetScoreWidg _returnvalue_2))
  ;[1 1 1] Adjust score for new level
  (bind _returnvalue_3 (Game|GetCurrentLevelName true))
  (if (and (Utilities|Enum|Equal(Enum) _returnvalue_3 "ShootingSceneRed") (< (Variables|Default|GetScoreVal) 10))
    (Variables|Default|SetScoreVal 10))
  ;[1 1 1] Displays score
  (Default|UpdateScore _output_get (Utilities|Text|ToText(String) (Utilities|String|Append "Score: " (Utilities|String|ToString(Text) (Utilities|Text|ToText(Integer) (Variables|Default|GetScoreVal))))))
  (UserInterface|Viewport|AddtoViewport _output_get 0)
  ;[1 1 1] Try to load a save game
  (bind _returnvalue_4 (SaveGame|LoadGamefromSlot "HighScore" :!label _label))
  (bind _assaved_score (Utilities|Casting|CastToSavedScore _returnvalue_4)
    (:then
      ;[1 1 1] Read saved score
      (bind _output_get_2 (Variables|Default|SetSavedScore _assaved_score))
      (bind _score (Default|ReadScore _output_get_2))
      (Default|SetHighScore (Variables|Default|GetScoreWidg) (Utilities|Text|ToText(String) (Utilities|String|Append "High Score: " (Utilities|String|ToString(Integer) _score))))
      ;[1 1 1] Spawn initial sphere
      (bind _returnvalue_5 (Game|SpawnActorfromClass "/Script/Engine.StaticMeshActor" (Math|Conversions|ToTransform(Vector) (Math|Vector|MakeVector 7.8e+02 (- (Math|Conversions|ToFloat(Integer) (Variables|Default|GetSpawnY)) 6e+02) 3.1e+02)) "Undefined" 0 0))
      (bind _returnvalue_6 (AddComponent|AddStaticMeshComponent _returnvalue_5 false))
      (Variables|Default|SetSpawnedSphere _returnvalue_5)
      (Variables|Default|SetSphereMesh _returnvalue_6)
      ;[1 1 1] Update spawn coordinate
      (Variables|Default|SetSpawnY (Math|Float|Truncate (Math|Float|%(Float) (+ (Math|Conversions|ToFloat(Integer) (Variables|Default|GetSpawnY)) 6e+02) 1.8e+03))))
    (:CastFailed
      (bind _returnvalue_7 (SaveGame|CreateSaveGameObject "/Game/BaseWorld/SavedScore.SavedScore_C"))
      (SaveGame|SaveGametoSlot _returnvalue_7 "HighScore")
      (goto _label))))

(event EventEndPlay
  (params (EndPlayReason :type EEndPlayReason%20Enum :default "Destroyed"))
  (bind _savedscore (Variables|Default|GetSavedScore))
  ;[1 1 1] Save at end
  (Default|SetScore _savedscore (Variables|Default|GetScoreVal))
  (SaveGame|SaveGametoSlot _savedscore "HighScore"))

(event EventTick
  (params (DeltaSeconds :type Float%20%28single-precision%29))
  (bind _returnvalue (Game|GetPlayerController 0))
  (bind (_locationx _locationy) (Game|Player|GetMousePosition _returnvalue))
  ;[1 1 1] Determine if we click the sphere
  (if (Math|Boolean|ANDBoolean (Math|Float|InRange(Float) _locationy (- (.Y (Math|Vector2D|BreakVector2D (.ScreenPosition (Class|GameplayStatics|ProjectWorldtoScreen _returnvalue (Transformation|GetWorldLocation (Variables|Default|GetSphereMesh)) false)))) 35.0) (+ (.Y (Math|Vector2D|BreakVector2D (.ScreenPosition (Class|GameplayStatics|ProjectWorldtoScreen _returnvalue (Transformation|GetWorldLocation (Variables|Default|GetSphereMesh)) false)))) 35.0)) (Math|Float|InRange(Float) _locationx (- (.X (Math|Vector2D|BreakVector2D (.ScreenPosition (Class|GameplayStatics|ProjectWorldtoScreen _returnvalue (Transformation|GetWorldLocation (Variables|Default|GetSphereMesh)) false)))) 35.0) (+ (.X (Math|Vector2D|BreakVector2D (.ScreenPosition (Class|GameplayStatics|ProjectWorldtoScreen _returnvalue (Transformation|GetWorldLocation (Variables|Default|GetSphereMesh)) false)))) 35.0)) (Game|Player|IsInputKeyDown _returnvalue "LeftMouseButton"))
    ;[1 1 1] Destroy the sphere
    (Actor|DestroyActor (Variables|Default|GetSpawnedSphere))
    ;[1 1 1] Update Score
    (bind _output_get (Variables|Default|SetScoreVal (+ (Variables|Default|GetScoreVal) 1)))
    (Default|UpdateScore (Variables|Default|GetScoreWidg) (Utilities|Text|ToText(String) (Utilities|String|Append "Score: " (Utilities|String|ToString(Text) (Utilities|Text|ToText(Integer) _output_get)))))
    ;[1 1 1] Do we need to change level?
    (bind _returnvalue_2 (Game|GetCurrentLevelName true))
    (if (and (Utilities|Enum|Equal(Enum) _returnvalue_2 "ShootingSceneBlue") (>= (Variables|Default|GetScoreVal) 10))
      ;[1 1 1] Change level
      (Game|OpenLevel(byName) "ShootingSceneRed")
      (else
        ;[1 1 1] Spawn sphere
        (bind _returnvalue_3 (Game|SpawnActorfromClass "/Script/Engine.StaticMeshActor" (Math|Conversions|ToTransform(Vector) (Math|Vector|MakeVector 7.8e+02 (- (Math|Conversions|ToFloat(Integer) (Variables|Default|GetSpawnY)) 6e+02) 3.1e+02)) "Undefined" 0 0))
        (bind _returnvalue_4 (AddComponent|AddStaticMeshComponent _returnvalue_3 false))
        (Variables|Default|SetSpawnedSphere _returnvalue_3)
        (Variables|Default|SetSphereMesh _returnvalue_4)
        ;[1 1 1] Update spawn coordinate
        (Variables|Default|SetSpawnY (Math|Float|Truncate (Math|Float|%(Float) (+ (Math|Conversions|ToFloat(Integer) (Variables|Default|GetSpawnY)) 6e+02) 1.8e+03)))))))

(fn ConstructionScript)